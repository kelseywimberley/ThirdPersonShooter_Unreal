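; BP_Pickup is a pickup actor that shows a text prompt while the third-person character overlaps it.
; Overlap registers it as the character's CurrentPickup, and any end overlap hides the text and clears that reference without checking which actor left.
; While overlapped, Tick rotates the text to face the character's follow camera.
; PickUpItem only destroys the actor and is not called within this Blueprint.
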(event Collision|EventActorBeginOverlap
  (params (OtherActor :type Actor%20Object%20Reference))
  (bind _asbp_third_person_character (Utilities|Casting|CastToBP_ThirdPersonCharacter OtherActor))
  (Variables|Default|SetPlayerCharacter _asbp_third_person_character)
  (Variables|Default|SetOverlap? true)
  (Rendering|SetVisibility (Variables|Default|GetTextRender) true false)
  (Variables|/Game/ThirdPerson/Blueprints/BP_ThirdPersonCharacter.BP_ThirdPersonCharacter_C|SetCurrentPickup _asbp_third_person_character self))

(event EventTick
  (params (DeltaSeconds :type Float%20%28single-precision%29))
  (bind _textrender (Variables|Default|GetTextRender))
  (if (Variables|Default|GetOverlap?)
    (Transformation|SetWorldRotation _textrender (Math|Rotator|FindLookatRotation (Transformation|GetWorldLocation _textrender) (Transformation|GetWorldLocation (Variables|/Game/ThirdPerson/Blueprints/BP_ThirdPersonCharacter.BP_ThirdPersonCharacter_C|GetFollowCamera (Variables|Default|GetPlayerCharacter)))) false false)))

(event Collision|EventActorEndOverlap
  (params (OtherActor :type Actor%20Object%20Reference))
  (Variables|Default|SetOverlap? false)
  (Rendering|SetVisibility (Variables|Default|GetTextRender) false false)
  (Variables|/Game/ThirdPerson/Blueprints/BP_ThirdPersonCharacter.BP_ThirdPersonCharacter_C|SetCurrentPickup (Variables|Default|GetPlayerCharacter) 0))

(fn ConstructionScript)

(fn PickUpItem
  (Actor|DestroyActor))