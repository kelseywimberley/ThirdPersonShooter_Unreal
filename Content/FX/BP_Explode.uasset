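; BP_Explode is a short-lived field system actor that breaks and scatters physics-field-driven destructibles as an explosion.
; On BeginPlay it applies external cluster strain with no falloff within the Sphere component's scaled radius to fracture clusters.
; It then applies a radial linear velocity from the sphere's center, scaled by the FieldMagnitude variable, and destroys itself after a brief delay.
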(event Custom|Break
  (bind _sphere (Variables|Default|GetSphere))
  (bind _fieldsystemcomponent (Variables|Field|GetFieldSystemComponent))
  (bind _returnvalue (Transformation|GetWorldLocation _sphere))
  (Class|FieldSystemComponent|ApplyPhysicsField _fieldsystemcomponent true "Field_ExternalClusterStrain" 0 (Field|SetRadialFalloff (Variables|Default|GetRadialFalloff) 5e+05 0.0 1.0 0.0 (Components|Sphere|GetScaledSphereRadius _sphere) _returnvalue "Field_FallOff_None"))
  (Class|FieldSystemComponent|ApplyPhysicsField _fieldsystemcomponent true "Field_LinearVelocity" 0 (Field|SetRadialVector (Variables|Default|GetRadialVector) (Variables|Default|GetField%20Magnitude) _returnvalue))
  (Utilities|FlowControl|Delay 0.2)
  (Actor|DestroyActor))

(event EventBeginPlay
  (CallFunction|Break))

(fn ConstructionScript)